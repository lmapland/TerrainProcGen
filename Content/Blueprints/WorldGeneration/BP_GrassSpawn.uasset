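; BP_GrassSpawn is a world-generation actor that sets up instanced mesh components for grass and foliage.
; On BeginPlay it creates one Instanced Static Mesh component per FoliageTypes entry, assigns that entry's mesh and stores it in FoliageComponents.
; After a short delay it enables actor tick, though this graph has no active Tick logic and adds no instances itself.
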(event EventBeginPlay
  (CallFunction|InitializeFoliageTypes)
  (Utilities|FlowControl|Delay 1.5)
  (Actor|Tick|SetActorTickEnabled true))

(event Collision|EventActorBeginOverlap
  (params (OtherActor :type Actor%20Object%20Reference)))

(event EventTick
  (params (DeltaSeconds :type Float%20%28single-precision%29)))

(fn ConstructionScript)

(fn InitializeFoliageTypes
  (for _array_element (Variables|Default|GetFoliageTypes)
    (bind _returnvalue (AddComponent|AddInstancedStaticMeshComponent false))
    (bind _output_get (LocalVariables|SetISM _returnvalue))
    (Components|StaticMesh|SetStaticMesh _output_get (Variables|/Script/Foliage.FoliageType_InstancedStaticMesh|GetMesh _array_element))
    (Utilities|Array|Add (Variables|Default|GetFoliageComponents) _output_get)))