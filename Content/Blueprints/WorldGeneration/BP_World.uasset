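; World actor that streams procedural terrain tiles and instanced foliage around the player.
; A looping timer queues nearby tiles, generates the closest asynchronously, draws it when ready and lifts fallen players.
; Terrain physics-state creation triggers foliage placement from section vertices, then frees the generator.
; Core generation calls are defined outside this graph; Blueprint versions (layered Perlin height, border-trimmed normals, trace-placed clusters with instance reuse) remain unused.
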(event Custom|SpawnTilesAroundPlayer
  (bind (_xstart _xend _ystart _yend) (CallFunction|GetTilesAroundPlayerBP))
  (bind _returnvalue (Game|GetPlayerCharacter 0))
  (bind _returnvalue_2 (Transformation|GetActorLocation _returnvalue))
  (if (< (.z (Transformation|GetActorLocation _returnvalue)) -3e+03)
    (Transformation|SetActorLocation _returnvalue (Math|Vector|MakeVector (.x _returnvalue_2) (.y _returnvalue_2) 1.5e+03) false false))
  (if (Variables|Default|GetbGeneratorBusy)
    (if (Variables|Default|GetbTileDataReady)
      (bind _returnvalue_3 (Class|WorldGenerator|DrawTile))
      (Variables|Default|SetGeneratedMeshIndex _returnvalue_3))
    (else
      (for _index (range _ystart _yend)
        (for _index_2 (range _xstart _xend)
          (bind _isnotgenerated (CallFunction|TileIsNotGenerated _index_2 _index (Variables|Default|GetMeshSectionIndex)))
          (if _isnotgenerated
            _)))
      (bind _returnvalue_4 (Class|WorldGenerator|GetClosestQueuedTile))
      (if (== (.Value (Utilities|Map|Find (Variables|Default|GetQueuedTiles) _returnvalue_4)) -1)
        (Class|WorldGenerator|GenerateTerrainAsync (.X (Utilities|Struct|BreakIntPoint _returnvalue_4)) (.Y (Utilities|Struct|BreakIntPoint _returnvalue_4)))))))

(event Custom|GenerateFoliageTile
  (params (TerrainMeshSectionIndex :type Integer))
  (bind _vertices (Class|KismetProceduralMeshLibrary|GetSectionfromProceduralMesh (Variables|Default|GetTerrainMesh) TerrainMeshSectionIndex))
  (bind _output_get (Variables|Default|SetFoliagePoints _vertices))
  (for _array_element _output_get
    (Class|WorldGenerator|AddFoliageInstances (+ _array_element (Transformation|GetActorLocation))))
  (CallFunction|RefreshFoliage))

(event Custom|OnPhysicsStateChanged
  (params (ChangedComponent :type Primitive%20Component%20Object%20Reference) (StateChange :type EComponentPhysicsStateChange%20Enum :default "Created"))
  (switch Utilities|FlowControl|Switch|SwitchonEComponentPhysicsStateChange StateChange
    (:Created
      (if (> (Variables|Default|GetGeneratedMeshIndex) -1)
        (CallFunction|GenerateFoliageTile (Variables|Default|GetGeneratedMeshIndex))
        (Variables|Default|SetbGeneratorBusy false)
        (Variables|Default|SetGeneratedMeshIndex -1)))))

(event EventBeginPlay
  ;[1 1 1] Handle whether foliage should be random or not and set seed as appropriate
  (if (Variables|Default|GetRandomizeFoliage)
    (Variables|Default|SetInitialFoliageSeed (Math|Random|RandomIntegerinRange 0 1000)))
  (Variables|Default|SetFoliageSeed (Math|Random|MakeRandomStream (Variables|Default|GetInitialFoliageSeed)))
  (Class|WorldGenerator|InitializeFoliageTypes)
  (CallFunction|SpawnTilesAroundPlayer)
  (Utilities|Time|SetTimerbyFunctionName 0 "SpawnTilesAroundPlayer" 0.1 true)
  (EventDispatchers|BindEventtoOnComponentPhysicsStateChanged (Variables|Default|GetTerrainMesh) (delegate Custom|OnPhysicsStateChanged)))

(event Collision|EventActorBeginOverlap
  (params (OtherActor :type Actor%20Object%20Reference)))

(event EventTick
  (params (DeltaSeconds :type Float%20%28single-precision%29)))

(event EventInitializeFoliageTypes
  (for _array_element (Variables|Default|GetFoliageTypes)
    (bind _returnvalue (AddComponent|AddInstancedStaticMeshComponent false))
    (Components|StaticMesh|SetStaticMesh _returnvalue (Variables|/Script/Foliage.FoliageType_InstancedStaticMesh|GetMesh _array_element))
    (Utilities|Array|Add (Variables|Default|GetFoliageComponents) _returnvalue))
  (Development|PrintString (Utilities|String|Append (Utilities|String|ToString(Integer) (Utilities|Array|Length (Variables|Default|GetFoliageTypes))) ", " (Utilities|String|ToString(Integer) (Utilities|Array|Length (Variables|Default|GetFoliageComponents))))))

(fn ConstructionScript)

(fn GenerateTerrainBP
  (params (SectionIndexX :type Integer) (SectionIndexY :type Integer))
  (bind _xvertexcount (Variables|Default|GetXVertexCount))
  (bind _triangles (LocalVariables|GetTriangles))
  (bind _cellsize (Variables|Default|GetCellSize))
  (bind _cellsize_2 (Variables|Default|GetCellSize))
  (bind _triangles_2 (LocalVariables|GetTriangles))
  (bind _terrainmesh (Variables|Default|GetTerrainMesh))
  (bind _meshsectionindex (Variables|Default|GetMeshSectionIndex))
  (bind _returnvalue (+ _xvertexcount 2))
  (LocalVariables|SetOffset (Math|Vector|MakeVector (Math|Conversions|ToFloat(Integer) (* SectionIndexX (* (- (Variables|Default|GetXVertexCount) 1) _cellsize_2))) (Math|Conversions|ToFloat(Integer) (* SectionIndexY (* (- (Variables|Default|GetYVertexCount) 1) _cellsize_2))) 0.0))
  (for _index (range -1 (Variables|Default|GetYVertexCount))
    (for _index_2 (range -1 (Variables|Default|GetXVertexCount))
      (bind _returnvalue_2 (Utilities|Array|Add (LocalVariables|GetVertices) (Math|Vector|MakeVector (+ (* _index_2 _cellsize) (.x (LocalVariables|GetOffset))) (+ (* _index _cellsize) (.y (LocalVariables|GetOffset))) (CallFunction|GenHeightBP (+ (* _index_2 _cellsize) (.x (LocalVariables|GetOffset))) (+ (* _index _cellsize) (.y (LocalVariables|GetOffset)))))))
      (Utilities|Array|Add (LocalVariables|GetUVs) (Math|Vector2D|MakeVector2D (.RetX (|CalculateUVOffset _index_2 _index)) (.RetY (|CalculateUVOffset _index_2 _index))))))
  (for _index_3 (range 0 (Variables|Default|GetYVertexCount))
    (for _index_4 (range 0 (Variables|Default|GetXVertexCount))
      (Utilities|Array|Add _triangles_2 (+ _index_4 (* _index_3 _returnvalue)))
      (Utilities|Array|Add _triangles_2 (+ (+ _index_4 (* _index_3 _returnvalue)) _returnvalue))
      (Utilities|Array|Add _triangles_2 (+ (+ _index_4 (* _index_3 _returnvalue)) 1))
      (Utilities|Array|Add _triangles (+ (+ _index_4 (* _index_3 _returnvalue)) _returnvalue))
      (Utilities|Array|Add _triangles (+ (+ (+ _index_4 (* _index_3 _returnvalue)) _returnvalue) 1))
      (Utilities|Array|Add _triangles (+ (+ _index_4 (* _index_3 _returnvalue)) 1))))
  (bind (_outvertices _outtriangles _outnormals _outuvs _outtangents) (CallFunction|GetSubsetBP (LocalVariables|GetVertices) (LocalVariables|GetTriangles) (LocalVariables|GetUVs)))
  (Class|ProceduralMeshComponent|CreateMeshSectionLinearColor _terrainmesh _meshsectionindex _outvertices _outtriangles _outnormals _outuvs 0 0 0 0 _outtangents true false)
  (bind _terrainmaterial (Variables|Default|GetTerrainMaterial)
    (:then
      (Rendering|Material|SetMaterial _terrainmesh _meshsectionindex _terrainmaterial)
      (Math|Integer|IncrementInt (Variables|Default|GetMeshSectionIndex)))
    (:else)))

(fn GenHeightBP
  (params (InX :type Float%20%28double-precision%29) (InY :type Float%20%28double-precision%29))
  (return (+ (CallFunction|GenerateHeightLayerBP InX InY (LocalVariables|GetScaleLarge) (LocalVariables|GetAmplitude)) (CallFunction|GenerateHeightLayerBP InX InY (LocalVariables|GetScaleMedium) (LocalVariables|GetAmplitudeMedium)) (CallFunction|GenerateHeightLayerBP InX InY (LocalVariables|GetScaleSmall) (LocalVariables|GetAmplitudeSmall)))))

(fn GenerateHeightLayerBP
  (params (InX :type Float%20%28double-precision%29) (InY :type Float%20%28double-precision%29) (InScale :type Float%20%28double-precision%29) (InAmplitude :type Float%20%28double-precision%29))
  (return (* (* (Class|KismetMathLibrary|PerlinNoise1D (+ (* InX InScale) 0.1)) (Class|KismetMathLibrary|PerlinNoise1D (+ (* InY InScale) 0.1))) InAmplitude)))

(fn GetPlayerPositionIndexBP
  (bind _returnvalue (Game|GetPlayerCharacter 0))
  (bind _cellsize (Variables|Default|GetCellSize))
  (bind _returnvalue_2 (Transformation|GetActorLocation _returnvalue))
  (Utilities|IsValid _returnvalue
    (:Is%20Valid
      (return (Math|Float|Truncate (/ (.x _returnvalue_2) (* _cellsize (- (Variables|Default|GetXVertexCount) 1)))) (Math|Float|Truncate (/ (.y _returnvalue_2) (* _cellsize (- (Variables|Default|GetYVertexCount) 1))))))
    (:Is%20Not%20Valid
      (return 0 0))))

(fn GetTilesAroundPlayerBP
  (bind (_playerx _playery) (CallFunction|GetPlayerPositionIndexBP))
  (bind _numbersectionsx (Variables|Default|GetNumberSectionsX))
  (bind _numbersectionsy (Variables|Default|GetNumberSectionsY))
  (bind _returnvalue (/ _numbersectionsx 2))
  (bind _returnvalue_2 (/ _numbersectionsy 2))
  (bind _returnvalue_3 (- _playery _returnvalue_2))
  (bind _returnvalue_4 (- _playerx _returnvalue))
  (return _returnvalue_4 (+ _returnvalue_4 _numbersectionsx -1) _returnvalue_3 (+ _returnvalue_3 _numbersectionsy -1)))

(fn GetSubsetBP
  (params (InVertices :type Array%20of%20Vectors) (InTriangles :type Array%20of%20Integers) (InUVs :type Array%20of%20Vector%202D%20Structures))
  (bind _yvertexcount (Variables|Default|GetYVertexCount))
  (bind _xvertexcount (Variables|Default|GetXVertexCount))
  (bind _triangles (LocalVariables|GetTriangles))
  (bind _triangles_2 (LocalVariables|GetTriangles))
  (bind _xvertexcount_2 (Variables|Default|GetXVertexCount))
  (bind (_normals _tangents) (Class|KismetProceduralMeshLibrary|CalculateTangentsforMesh InVertices InTriangles InUVs))
  (bind _output_get (LocalVariables|SetBigNormals _normals))
  (bind _output_get_2 (LocalVariables|SetBigTangents _tangents))
  (for _index (range -1 _yvertexcount)
    (for _index_2 (range -1 _xvertexcount_2)
      (if (Math|Boolean|ANDBoolean (> _index_2 -1) (< _index_2 _xvertexcount_2) (> _index -1) (< _index _yvertexcount))
        (Utilities|FlowControl|Sequence
          (:then_0
            (Utilities|Array|Add (LocalVariables|GetVertices) (Utilities|Array|Get(acopy) InVertices (LocalVariables|GetIndex)))
            (Utilities|Array|Add (LocalVariables|GetUVs) (Utilities|Array|Get(acopy) InUVs (LocalVariables|GetIndex)))
            (Utilities|Array|Add (LocalVariables|GetSubNormals) (Utilities|Array|Get(acopy) (LocalVariables|GetBigNormals) (LocalVariables|GetIndex)))
            (Utilities|Array|Add (LocalVariables|GetSubTangents) (Utilities|Array|Get(acopy) (LocalVariables|GetBigTangents) (LocalVariables|GetIndex))))
          (:then_1
            (Math|Integer|IncrementInt (LocalVariables|GetIndex) :!label _label)))
        (else
          (goto _label)))))
  (for _index_3 (range 0 (- (Variables|Default|GetYVertexCount) 2))
    (for _index_4 (range 0 (- (Variables|Default|GetXVertexCount) 2))
      (Utilities|Array|Add _triangles_2 (+ _index_4 (* _index_3 _xvertexcount)))
      (Utilities|Array|Add _triangles_2 (+ (+ _index_4 (* _index_3 _xvertexcount)) _xvertexcount))
      (Utilities|Array|Add _triangles_2 (+ (+ _index_4 (* _index_3 _xvertexcount)) 1))
      (Utilities|Array|Add _triangles (+ (+ _index_4 (* _index_3 _xvertexcount)) _xvertexcount))
      (Utilities|Array|Add _triangles (+ (+ (+ _index_4 (* _index_3 _xvertexcount)) _xvertexcount) 1))
      (Utilities|Array|Add _triangles (+ (+ _index_4 (* _index_3 _xvertexcount)) 1))))
  (return (LocalVariables|GetVertices) (LocalVariables|GetTriangles) (LocalVariables|GetSubNormals) (LocalVariables|GetUVs) (LocalVariables|GetSubTangents)))

(fn TileIsNotGenerated
  (params (InSectionX :type Integer) (InSectionY :type Integer) (InMeshSection :type Integer))
  ;[1 1 1] Don't generate the tile if the tile location is already outside the player's Discard Distance
  (bind _returnvalue (Class|WorldGenerator|GetTileLocation (Utilities|Struct|MakeIntPoint InSectionX InSectionY)))
  (bind _returnvalue_2 (Class|WorldGenerator|GetPlayerLocation))
  (if (> (Math|Vector|Distance2D(Vector) (Math|Conversions|ToVector2D(Vector) _returnvalue_2) _returnvalue) (Variables|Default|GetTileDiscardDistance))
    _
    (elif (.ReturnValue (Utilities|Map|Find (Variables|Default|GetQueuedTiles) (Utilities|Struct|MakeIntPoint InSectionX InSectionY)))
      _
      (else
        (Utilities|Map|Add (Variables|Default|GetQueuedTiles) (Utilities|Struct|MakeIntPoint InSectionX InSectionY) -1)
        (return true))))
  (return false))

(fn AddFoliageInstances2
  (params (InstanceTransform_Location :type Vector))
  ;[1 1 1] Don't spawn primary foliage instance if Z is too low
  (if (> (.Z (Math|Vector|BreakVector InstanceTransform_Location)) 5e+01)
    ;[1 1 1] Choose to spawn foliage or not based on Foliage Spawn Percentage
    (if (< (Math|Random|RandomIntegerinRange 0 100) (Variables|Default|GetFoliageSpawnPercentage))
      (for _index (range 1 (Math|Random|RandomIntegerinRange 0 (Variables|Default|GetMaxClusterSize)))
        ;[1 1 1] Get Cluster foliage instance's X and Y coords
        (bind _returnvalue (CallFunction|RandomizeFoliageOffset _index))
        (bind _returnvalue_2 (CallFunction|RandomizeFoliageOffset _index))
        (bind (_outhit _returnvalue_3) (Collision|LineTraceByChannel (+ (+ InstanceTransform_Location (Math|Vector|MakeVector _returnvalue _returnvalue_2 0.0)) "0.000000,0.000000,2000.000000") (+ (+ InstanceTransform_Location (Math|Vector|MakeVector _returnvalue _returnvalue_2 0.0)) "0.000000,0.000000,-2000.000000") "TraceTypeQuery1" false 0 "None" false))
        (if _returnvalue_3
          _)))))

(fn RandomizeFoliageOffset
  (params (Index :type Integer))
  (bind _instanceoffset (Variables|Default|GetInstanceOffset))
  (return (* (* Index (Math|Random|RandomIntegerinRangefromStream (Variables|Default|GetFoliageSeed) _instanceoffset (+ _instanceoffset (Variables|Default|GetInstanceOffsetVariation)))) (Math|Float|SelectFloat -1.0 1.0 (Math|Random|RandomBoolfromStream (Variables|Default|GetFoliageSeed))))))

(fn RemoveFoliageTile
  (params (TileIndex :type Integer))
  (bind _returnvalue (Transformation|GetActorLocation))
  (bind _amplitudelarge (Variables|Default|GetAmplitudeLarge))
  (bind _amplitudemedium (Variables|Default|GetAmplitudeMedium))
  (bind _amplitudesmall (Variables|Default|GetAmplitudeSmall))
  (bind _returnvalue_2 (+ _amplitudelarge _amplitudemedium _amplitudesmall))
  (bind _vertices (Class|KismetProceduralMeshLibrary|GetSectionfromProceduralMesh (Variables|Default|GetTerrainMesh) TileIndex))
  (if (> (Utilities|Array|LastIndex _vertices) 0)
    (LocalVariables|SetFirst (+ (Utilities|Array|Get(acopy) _vertices) _returnvalue))
    (LocalVariables|SetLast (+ (Utilities|Array|Get(acopy) _vertices (Utilities|Array|LastIndex _vertices)) _returnvalue))
    (for _array_element (Variables|Default|GetFoliageComponents)
      (LocalVariables|SetOverlappingInstances (Class|InstancedStaticMeshComponent|GetInstancesOverlappingBox _array_element (Math|Box|MakeBox (Math|Vector|MakeVector (.x (LocalVariables|GetFirst)) (.y (LocalVariables|GetFirst)) (* _returnvalue_2 -1.0)) (Math|Vector|MakeVector (.x (LocalVariables|GetLast)) (.y (LocalVariables|GetLast)) _returnvalue_2)) true))
      (if (.ReturnValue (Utilities|Map|Find (Variables|Default|GetReplaceableFoliagePool) _array_element))
        (Utilities|Array|AppendArray (Utilities|Struct|BreakFoliageInstanceData (.Value (Utilities|Map|Find (Variables|Default|GetReplaceableFoliagePool) _array_element))) (LocalVariables|GetOverlappingInstances)))
      (Utilities|Map|Add (Variables|Default|GetReplaceableFoliagePool) 0 (Utilities|Struct|MakeFoliageInstanceData (LocalVariables|GetOverlappingInstances))))
    (return true)
    (else
      (Development|PrintString "Tile Index is too big!"))))

(fn AddRelevantFoliageInstances
  (params (Location :type Vector))
  (bind _scalevariationmultiplier (Variables|Default|GetScaleVariationMultiplier))
  (bind _foliageseed (Variables|Default|GetFoliageSeed))
  (bind _instancescale (Variables|Default|GetInstanceScale))
  (bind _returnvalue (* _scalevariationmultiplier -1.0))
  (bind _returnvalue_2 (Math|Random|RandomFloatinRangefromStream _foliageseed _returnvalue _scalevariationmultiplier))
  (bind _returnvalue_3 (+ _returnvalue_2 1.0))
  (bind _returnvalue_4 (* _instancescale _returnvalue_3))
  (for (_array_element _array_index) (Variables|Default|GetFoliageTypes)
    (LocalVariables|SetActiveFoliageTypeIndex _array_index)
    (LocalVariables|SetActiveFoliageType _array_element)
    ;[1 1 1] Choose to spawn foliage or not based on Foliage Spawn Percentage
    (if (< (Math|Random|RandomIntegerinRangefromStream (Variables|Default|GetFoliageSeed) 0 100) (Variables|Default|GetFoliageSpawnPercentage))
      ;[1 1 1] Don't spawn primary foliage instance if Z is outside spawn range
      (if (Math|Float|InRange(Float) (.Z (Math|Vector|BreakVector Location)) (.min (Variables|/Script/Foliage.FoliageType|GetHeight (LocalVariables|GetActiveFoliageType))) (.max (Variables|/Script/Foliage.FoliageType|GetHeight (LocalVariables|GetActiveFoliageType))))
        (for _index (range 0 (Math|Random|RandomIntegerinRangefromStream (Variables|Default|GetFoliageSeed) 0 (Variables|Default|GetMaxClusterSize)))
          ;[1 1 1] Get Cluster foliage instance's X and Y coords
          (bind _returnvalue_5 (CallFunction|RandomizeFoliageOffset _index))
          (bind _returnvalue_6 (CallFunction|RandomizeFoliageOffset _index))
          (bind (_outhit _returnvalue_7) (Collision|LineTraceByChannel (+ (+ Location (Math|Vector|MakeVector _returnvalue_5 _returnvalue_6 0.0)) "0.000000,0.000000,2000.000000") (+ (+ Location (Math|Vector|MakeVector _returnvalue_5 _returnvalue_6 0.0)) "0.000000,0.000000,-2000.000000") "TraceTypeQuery1" false 0 "None" false))
          (if _returnvalue_7
            (if (== (.HitComponent (Collision|BreakHitResult _outhit)) (Variables|Default|GetTerrainMesh))
              ;[1 1 1] Don't spawn primary foliage instance if Z is outside spawn range
              (if (Math|Float|InRange(Float) (.Z (Math|Vector|BreakVector (.Location (Collision|BreakHitResult _outhit)))) (.min (Variables|/Script/Foliage.FoliageType|GetHeight (LocalVariables|GetActiveFoliageType))) (.max (Variables|/Script/Foliage.FoliageType|GetHeight (LocalVariables|GetActiveFoliageType))))
                (bind _output_get (LocalVariables|SetReplaceablePool (.instances (.Value (Utilities|Map|Find (Variables|Default|GetReplaceableFoliagePool) (Utilities|Array|Get(acopy) (Variables|Default|GetFoliageComponents) (LocalVariables|GetActiveFoliageTypeIndex)))))))
                (if (and (.ReturnValue (Utilities|Map|Find (Variables|Default|GetReplaceableFoliagePool) (Utilities|Array|Get(acopy) (Variables|Default|GetFoliageComponents) (LocalVariables|GetActiveFoliageTypeIndex)))) (> (Utilities|Array|Length _output_get) 0))
                  (Components|InstancedStaticMesh|UpdateInstanceTransform (Utilities|Array|Get(acopy) (Variables|Default|GetFoliageComponents) (LocalVariables|GetActiveFoliageTypeIndex)) (Utilities|Array|Get(acopy) _output_get (Utilities|Array|LastIndex _output_get)) (Math|Transform|MakeTransform (.Location (Collision|BreakHitResult _outhit)) (.rotation (.OutInstanceTransform (Components|InstancedStaticMesh|GetInstanceTransform (Utilities|Array|Get(acopy) (Variables|Default|GetFoliageComponents) (LocalVariables|GetActiveFoliageTypeIndex)) 0 false))) _returnvalue_4) true true false)
                  (Utilities|Array|RemoveIndex _output_get (Utilities|Array|LastIndex _output_get))
                  (Utilities|Map|Add (Variables|Default|GetReplaceableFoliagePool) (Utilities|Array|Get(acopy) (Variables|Default|GetFoliageComponents) (LocalVariables|GetActiveFoliageTypeIndex)) (Utilities|Struct|MakeFoliageInstanceData _output_get))
                  (else
                    (Components|InstancedStaticMesh|AddInstance (Utilities|Array|Get(acopy) (Variables|Default|GetFoliageComponents) (LocalVariables|GetActiveFoliageTypeIndex)) (Math|Transform|MakeTransform (.Location (Collision|BreakHitResult _outhit)) "0, 0, 0" _returnvalue_4) true)))))))))))

(fn RefreshFoliage
  (for _array_element (Variables|Default|GetFoliageComponents)
    (Components|InstancedStaticMesh|UpdateInstanceTransform _array_element 0 (.OutInstanceTransform (Components|InstancedStaticMesh|GetInstanceTransform _array_element 0 true)) true true false)))